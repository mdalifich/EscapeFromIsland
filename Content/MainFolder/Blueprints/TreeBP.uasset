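; TreeBP is a harvestable tree that the player chops with an axe to gain resources.
; When a BP_Axe overlaps its Capsule, it calls its destroy event.
; That event adds small random amounts, possibly zero, to the Lian and Wood counts on the MainPerson pawn of player 0, then destroys the tree actor.
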(event OnComponentBeginOverlap(Capsule)
  (params (OverlappedComponent :type Primitive%20Component%20Object%20Reference) (OtherActor :type Actor%20Object%20Reference) (OtherComp :type Primitive%20Component%20Object%20Reference) (OtherBodyIndex :type Integer) (bFromSweep :type Boolean) (SweepResult :type Hit%20Result%20Structure%20%28by%20ref%29))
  (Utilities|Casting|CastToBP_Axe OtherActor)
  (CallFunction|Destroy))

(event Custom|destroy
  (bind _asmain_person (Utilities|Casting|CastToMainPerson (Game|Player|GetPlayerPawn 0)))
  (Variables|/Game/MainFolder/Blueprints/MainPerson.MainPerson_C|Setlian _asmain_person (+ (Variables|/Game/MainFolder/Blueprints/MainPerson.MainPerson_C|Getlian _asmain_person) (Math|Random|RandomInteger 5)))
  (Variables|/Game/MainFolder/Blueprints/MainPerson.MainPerson_C|Setwood _asmain_person (+ (Variables|/Game/MainFolder/Blueprints/MainPerson.MainPerson_C|Getwood _asmain_person) (Math|Random|RandomInteger 3)))
  (Actor|DestroyActor))

(fn ConstructionScript)